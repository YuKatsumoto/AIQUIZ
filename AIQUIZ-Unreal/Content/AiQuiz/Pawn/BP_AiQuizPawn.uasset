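; AI quiz pawn that acts as a side-view player character, moving left and right with A/D or arrow keys and jumping with Space.
; Tick polls keys directly and integrates position and gravity in simplified 2D units, then scales them onto world Y/Z at fixed X.
; Ground is a math-only strip around the origin without collision; falling below it resets to center.
; All conditional logic uses branchless SelectFloat chains.
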(event `self.ReceiveTick`
  (params (DeltaSeconds :type "Float (single-precision)"))
  (bind _returnvalue (`GameplayStatics.GetPlayerController` 0))
  (bind _vely (`self.VelY`))
  (bind _playerx (`self.PlayerX`))
  (bind _playery (`self.PlayerY`))
  (bind _returnvalue_2 (<= _playery 0.0))
  (bind _returnvalue_3 (< _playery -8.0))
  (bind _returnvalue_4 (<= (`KismetMathLibrary.Abs` _playerx) 12.0))
  (bind _returnvalue_5 (and _returnvalue_2 _returnvalue_4))
  (set `self.AxisX` (+ (`KismetMathLibrary.SelectFloat` 1.0 0.0 (or (`PlayerController.IsInputKeyDown` _returnvalue "A") (`PlayerController.IsInputKeyDown` _returnvalue "Left"))) (`KismetMathLibrary.SelectFloat` -1.0 0.0 (or (`PlayerController.IsInputKeyDown` _returnvalue "D") (`PlayerController.IsInputKeyDown` _returnvalue "Right")))))
  (set `self.PlayerX` (+ _playerx (* (* (`self.AxisX`) 7.6) DeltaSeconds)))
  (set `self.VelY` (`KismetMathLibrary.SelectFloat` 7.0 _vely (and (`PlayerController.WasInputKeyJustPressed` _returnvalue "SpaceBar") (and _returnvalue_2 _returnvalue_4))))
  (set `self.VelY` (- _vely (* 18.0 DeltaSeconds)))
  (set `self.PlayerY` (+ _playery (* _vely DeltaSeconds)))
  (set `self.PlayerY` (`KismetMathLibrary.SelectFloat` 0.0 _playery _returnvalue_5))
  (set `self.VelY` (`KismetMathLibrary.SelectFloat` 0.0 _vely _returnvalue_5))
  (set `self.PlayerX` (`KismetMathLibrary.SelectFloat` 0.0 _playerx _returnvalue_3))
  (set `self.VelY` (`KismetMathLibrary.SelectFloat` 0.0 _vely _returnvalue_3))
  (set `self.PlayerY` (`KismetMathLibrary.SelectFloat` 0.0 _playery _returnvalue_3))
  (`self.K2_SetActorLocation` (`KismetMathLibrary.MakeVector` -800.0 (* _playerx -100.0) (* _playery 100.0))))

(fn `UserConstructionScript`)